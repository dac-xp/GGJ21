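; Top-down player character that moves on world axes, faces the cursor, fires tagged bullets, blinks and scans for a hidden target.
; BeginPlay spawns the target invisibly at a random point; scanning pulses a particle effect and reveals the target if within range.
; Tick handles aiming and held-button fire, with Delay-reset flags limiting fire rate and the impulse-driven blink dash.
; Overlapping enemy-tagged bullets reduces health; death only prints a message.
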(event `InputAction|scan`
  (params (Key :type "Key Structure"))
  (bind _scandistancetotarget (`self.ScanDistanceToTarget`))
  (bind _sphere (`/Game/LostItem/BP_Target.Sphere` (`self.Target`)))
  (bind (_returnvalue_roll _returnvalue_pitch) (`KismetMathLibrary.BreakRotator` (`KismetMathLibrary.Conv_VectorToRotator` (`KismetMathLibrary.InverseTransformLocation` (`SceneComponent.K2_GetComponentToWorld` (`self.CapsuleComponent`)) (`self.K2_GetActorLocation` (`self.Target`))))))
  (:`Pressed`
    (`|ExecutionSequence`
      (:`then_0`
        ;[1 1 1] spawn scanning emitter
        (bind _returnvalue (`GameplayStatics.SpawnEmitterAtLocation` "/Game/Player/Scanner/PS_ScanEffect.PS_ScanEffect" (`SceneComponent.K2_GetComponentLocation` (`self.CapsuleComponent`))))
        (`FXSystemComponent.SetFloatParameter` _returnvalue "ScanRadius" (* (`self.MaxScanDistance`) 2.5)))
      (:`then_1`
        ;[1 1 1] rotation relative to target position
        (set `self.ScanRotationToTarget` _returnvalue_pitch))
      (:`then_2`
        ;[1 1 1] distance to target
        (set `self.ScanDistanceToTarget` (`KismetMathLibrary.Vector_Distance` (`SceneComponent.K2_GetComponentLocation` (`self.CapsuleComponent`)) (`self.K2_GetActorLocation` (`self.Target`)))))
      (:`then_3`
        ;[1 1 1] check if target is in scan distance
        (if (> (`self.MaxScanDistance`) _scandistancetotarget)
          (`KismetSystemLibrary.Delay` 0.3)
          (`SceneComponent.SetVisibility` _sphere true false)
          (bind _returnvalue_2 (`GameplayStatics.SpawnEmitterAtLocation` "/Game/Player/Scanner/PS_ScanEffect.PS_ScanEffect" (`SceneComponent.K2_GetComponentLocation` _sphere)))
          (`FXSystemComponent.SetFloatParameter` _returnvalue_2 "ScanRadius" 800.0)
          (else
            (`KismetSystemLibrary.PrintString` (`KismetStringLibrary.Conv_DoubleToString` _scandistancetotarget))))))))

(event `InputAction|Blink`
  (params (Key :type "Key Structure"))
  (bind _charactermovement (`self.CharacterMovement`))
  (:`Pressed`
    ;[1 1 1] blink
    (if (`self.CanBlink`)
      (set `self.CanBlink` false)
      (bind _output_get (set `self.BlinkDirection` (`SceneComponent.GetForwardVector` (`self.CapsuleComponent`))))
      (bind _returnvalue (* _output_get 8000))
      (`CharacterMovementComponent.AddImpulse` _charactermovement _returnvalue true)
      (`KismetSystemLibrary.Delay` 0.1)
      (set `MovementComponent.Velocity` (* (`KismetMathLibrary.Normal` _output_get) (`KismetMathLibrary.FMin` (`CharacterMovementComponent.MaxFlySpeed` _charactermovement) (`KismetMathLibrary.VSize` _returnvalue))) (`self.CharacterMovement`))
      (`KismetSystemLibrary.Delay` 2.0)
      (set `self.CanBlink` true))))

(event `InputAxis|Horizontal Movement`
  (params (AxisValue :type "Float (single-precision)"))
  ;[1 1 1] move player
  (`self.AddMovementInput` (0.0 30.0 0.0) AxisValue true))

(event `InputAxis|Vertical Movement`
  (params (AxisValue :type "Float (single-precision)"))
  ;[1 1 1] move player
  (`self.AddMovementInput` (30.0 0.0 0.0) AxisValue true))

(event `self.ReceiveTick`
  (params (DeltaSeconds :type "Float (single-precision)"))
  (bind (_returnvalue_roll _returnvalue_pitch) (`KismetMathLibrary.BreakRotator` (`self.K2_GetActorRotation`)))
  (bind _capsulecomponent (`self.CapsuleComponent`))
  (bind (_returnvalue_roll_2 _returnvalue_pitch_2 _returnvalue_yaw) (`KismetMathLibrary.BreakRotator` (`KismetMathLibrary.FindLookAtRotation` (`self.K2_GetActorLocation`) (`.Location` (`GameplayStatics.BreakHitResult` (`PlayerController.GetHitResultUnderCursorByChannel` (`GameplayStatics.GetPlayerController` 0) "TraceTypeQuery1" true))))))
  ;[1 1 1] look at cursor
  (`SceneComponent.K2_SetWorldRotation` (`self.CapsuleComponent`) (`KismetMathLibrary.MakeRotator` _returnvalue_roll _returnvalue_pitch _returnvalue_yaw) false false)
  ;[1 1 1] fire bullets
  (if (and (`self.CanFire`) (`self.IsFiring`))
    (set `self.CanFire` false)
    (bind _returnvalue (`|SpawnActorFromClass` "/Game/Player/BP_Bullet.BP_Bullet_C" (`KismetMathLibrary.MakeTransform` (+ (`SceneComponent.K2_GetComponentLocation` _capsulecomponent) (* (`SceneComponent.GetForwardVector` _capsulecomponent) 50)) (`SceneComponent.K2_GetComponentRotation` _capsulecomponent)) "Undefined" "OverrideRootScale" null null))
    (bind _tags (`Actor.Tags` _returnvalue))
    (`KismetArrayLibrary.Array_Add` _tags "PlayerBullet")
    (set `Actor.Tags` _tags _returnvalue)
    (`KismetSystemLibrary.Delay` (/ 1.0 (`self.BulletsPerSecond`)))
    (set `self.CanFire` true)))

(event `InputAction|Fire`
  (params (Key :type "Key Structure"))
  ;[1 1 1] fire bullets
  (:`Pressed`
    (set `self.IsFiring` true))
  (:`Released`
    (set `self.IsFiring` false)))

(event `self.ReceiveBeginPlay`
  ;[1 1 1] show mouse cursor
  (set `PlayerController.bShowMouseCursor` true (`GameplayStatics.GetPlayerController` 0))
  ;[1 1 1] spawn target to find
  (bind _returnvalue (`|SpawnActorFromClass` "/Game/LostItem/BP_Target.BP_Target_C" (`KismetMathLibrary.MakeTransform` (`KismetMathLibrary.RandomPointInBoundingBox` (0.0 0.0 0.0) (5000.0 5000.0 0.0))) "Undefined" "OverrideRootScale" null null))
  (bind _output_get (set `self.Target` _returnvalue))
  (`SceneComponent.SetVisibility` (`/Game/LostItem/BP_Target.Sphere` _output_get) false false)
  ;[1 1 1] initialize player health
  (set `self.Health` (`self.MaxHealth`)))

(event `self.ReceiveActorBeginOverlap`
  (params (OtherActor :type "Actor Object Reference"))
  ;[1 1 1] inflict damage
  (if (`self.ActorHasTag` OtherActor "EnemyBullet")
    (bind _output_get (set `self.Health` (- (`self.Health`) 10)))
    ;[1 1 1] player dies
    (if (<= _output_get 0)
      (`KismetSystemLibrary.PrintString` "EXPLOSION! END GAME!"))))

(fn `UserConstructionScript`)