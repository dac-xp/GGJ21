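; Flying AI enemy character that shoots at the player and explodes when destroyed by player bullets.
; Overlaps with actors tagged PlayerBullet reduce health, and death unpossesses the controller, plays effects, spawns a drop and destroys the enemy.
; Attack spawns tagged bullets from left and right laser points while the player is alive, guarded by CanFire.
; UpdateFlySpeed exposes the movement component's maximum fly speed.
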(event `self.ReceiveBeginPlay`
  ;[1 1 1] initialize health
  (set `self.Health` (`self.MaxHealth`)))

(event `self.ReceiveActorBeginOverlap`
  (params (OtherActor :type "Actor Object Reference"))
  ;[1 1 1] inflict damage
  (bind _output_get (set `self.NewVar_1` (`self.K2_GetActorLocation` OtherActor)))
  (if (`self.ActorHasTag` OtherActor "PlayerBullet")
    (`self.K2_DestroyActor` OtherActor)
    (bind _output_get_2 (set `self.Health` (- (`self.Health`) 10)))
    (`GameplayStatics.PlaySoundAtLocation` "/Game/Sounds/tick_2.tick_2" _output_get (struct) 1.0 1.0 0.0 null null null)
    ;[1 1 1] enemy dies
    (if (<= _output_get_2 0)
      (bind _output_get_3 (set `self.NewVar_0` (`SceneComponent.K2_GetComponentLocation` (`self.Mesh`))))
      (`GameplayStatics.SpawnEmitterAtLocation` "/Game/Explosions/Particles/P_ImpactExplosion4.P_ImpactExplosion4" _output_get_3 (struct) (2.0 2.0 2.0))
      (`Controller.UnPossess` (`AIBlueprintHelperLibrary.GetAIController` null))
      (`|ExecutionSequence`
        (:`then_0`
          (`|SpawnActorFromClass` "/Game/Enemy/Drop.Drop_C" (`KismetMathLibrary.MakeTransform` _output_get_3) "Undefined" "OverrideRootScale" null null)
          (`self.K2_DestroyActor`))
        (:`then_1`
          (`GameplayStatics.PlaySoundAtLocation` "/Game/Sounds/explosion_002.explosion_002" _output_get_3 (struct) 1.0 1.0 0.0 null null null))))))

(fn `Attack`
  ;[1 1 1] fire bullets
  (bind _asbp_player_character (cast `/Game/Player/BP_PlayerCharacter` (`GameplayStatics.GetPlayerCharacter` 0)))
  (if (and (`self.CanFire`) (not (`/Game/Player/BP_PlayerCharacter.isDead` _asbp_player_character)))
    (set `self.CanFire` false)
    (`|ExecutionSequence`
      (:`then_0`
        (bind _returnvalue (`|SpawnActorFromClass` "/Game/Enemy/BP_EnemyBullet.BP_EnemyBullet_C" (`KismetMathLibrary.MakeTransform` (`SceneComponent.K2_GetComponentLocation` (`self.LaserRight`)) (`SceneComponent.K2_GetComponentRotation` (`self.CapsuleComponent`))) "Undefined" "OverrideRootScale" null null))
        (bind _tags (`Actor.Tags` _returnvalue))
        (`KismetArrayLibrary.Array_Add` _tags "EnemyBulletBullet")
        (set `Actor.Tags` _tags _returnvalue)
        (`GameplayStatics.PlaySoundAtLocation` "/Game/Sounds/shooting_005.shooting_005" (`SceneComponent.K2_GetComponentLocation` (`self.CapsuleComponent`)) (struct) 1.0 1.0 0.0 null null null)
        (set `self.CanFire` true))
      (:`then_1`
        (bind _returnvalue_2 (`|SpawnActorFromClass` "/Game/Enemy/BP_EnemyBullet.BP_EnemyBullet_C" (`KismetMathLibrary.MakeTransform` (`SceneComponent.K2_GetComponentLocation` (`self.LaserLeft`)) (`SceneComponent.K2_GetComponentRotation` (`self.CapsuleComponent`))) "Undefined" "OverrideRootScale" null null))
        (bind _tags_2 (`Actor.Tags` _returnvalue_2))
        (`KismetArrayLibrary.Array_Add` _tags_2 "EnemyBulletBullet")
        (set `Actor.Tags` _tags_2 _returnvalue_2)))))

(fn `Update Fly Speed`
  (params (NewFlySpeed :type "Float (double-precision)"))
  (set `CharacterMovementComponent.MaxFlySpeed` NewFlySpeed (`self.CharacterMovement`)))

(fn `UserConstructionScript`)